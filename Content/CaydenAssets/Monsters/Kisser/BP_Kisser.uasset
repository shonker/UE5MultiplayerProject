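; BP_Kisser is a monster that walks toward a randomly chosen MyBlasterCharacter on BeginPlay and performs a kill on overlap.
; The first overlap of any actor latches FoundTarget; if it is a MyBlasterCharacter, the victim snaps onto the monster, gets KissDeath set and loses movement.
; The kill animation then plays and the victim's camera boom length is set.
; The construction script attaches a Censor component to the mesh's face socket.
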(event EventBeginPlay
  (bind _outactors (Actor|GetAllActorsOfClass "/Game/Blueprints/Character/MyBlasterCharacter.MyBlasterCharacter_C"))
  (bind _output_get (Variables|Default|SetOut%20Actors _outactors))
  (AI|AIMoveTo self "0, 0, 0" (.OutItem (Utilities|Array|Random _output_get)) 5.0 false))

(event Collision|EventActorBeginOverlap
  (params (OtherActor :type Actor%20Object%20Reference))
  (if (not (Variables|Default|GetFoundTarget))
    (Variables|Default|SetFoundTarget true)
    (bind _asmy_blaster_character (Utilities|Casting|CastToMyBlasterCharacter OtherActor))
    (Transformation|SetActorLocationAndRotation _asmy_blaster_character (Transformation|GetActorLocation) (Transformation|GetActorRotation))
    (Variables|/Game/Blueprints/Character/MyBlasterCharacter.MyBlasterCharacter_C|SetKissDeath _asmy_blaster_character true)
    (Pawn|Components|CharacterMovement|DisableMovement (Variables|/Script/Engine.Character|GetCharacterMovement _asmy_blaster_character))
    (Components|Animation|PlayAnimation (Variables|Character|GetMesh) "/Game/CaydenAssets/Monsters/Kisser/Kisser_Anim_skele_Kill.Kisser_Anim_skele_Kill" false)
    (Variables|/Script/Engine.SpringArmComponent|SetTargetArmLength (Variables|/Game/Blueprints/Character/MyBlasterCharacter.MyBlasterCharacter_C|GetCamera%20Boom _asmy_blaster_character) 1e+02)))

(event EventTick
  (params (DeltaSeconds :type Float%20%28single-precision%29)))

(fn ConstructionScript
  (Transformation|AttachComponentToComponent (Variables|Default|Getcensor) (Variables|Character|GetMesh) "faceSocket" "KeepRelative" "KeepRelative" "KeepRelative" true))