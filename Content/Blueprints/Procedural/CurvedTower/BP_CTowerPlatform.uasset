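; BP_CTowerPlatform is a platform piece for the procedural curved tower that exposes a set of output points.
; Its construction script collects the relative transforms of eleven Output components into the OutputTransforms array, in a hand-wired order rather than numeric order.
; Output11 is left out of the array, and the event graph has no active logic.
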(event EventBeginPlay)

(event Collision|EventActorBeginOverlap
  (params (OtherActor :type Actor%20Object%20Reference)))

(event EventTick
  (params (DeltaSeconds :type Float%20%28single-precision%29)))

(fn ConstructionScript
  (Variables|Default|SetOutputTransforms (Utilities|Array|MakeArray (Transformation|GetRelativeTransform (Variables|Default|GetOutput5)) (Transformation|GetRelativeTransform (Variables|Default|GetOutput10)) (Transformation|GetRelativeTransform (Variables|Default|GetOutput6)) (Transformation|GetRelativeTransform (Variables|Default|GetOutput7)) (Transformation|GetRelativeTransform (Variables|Default|GetOutput8)) (Transformation|GetRelativeTransform (Variables|Default|GetOutput9)) (Transformation|GetRelativeTransform (Variables|Default|GetOutput4)) (Transformation|GetRelativeTransform (Variables|Default|GetOutput3)) (Transformation|GetRelativeTransform (Variables|Default|GetOutput)) (Transformation|GetRelativeTransform (Variables|Default|GetOutput1)) (Transformation|GetRelativeTransform (Variables|Default|GetOutput2)))))