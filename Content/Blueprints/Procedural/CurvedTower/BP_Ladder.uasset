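; Climbable ladder actor for MyBlasterCharacter, driven by collision with its Cube and Box components.
; Overlapping the Box switches the character's movement to Flying, and leaving restores Walking.
; Hitting the Cube adds movement input along the horizontal ladder-to-player direction plus a vertical term signed by camera pitch, so looking up or down sets climb direction.
; All events ignore InteractSphere, and the construction script sizes the Box from the Cube's scale.
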(event OnComponentBeginOverlap(Box)
  (params (OverlappedComponent :type Primitive%20Component%20Object%20Reference) (OtherActor :type Actor%20Object%20Reference) (OtherComp :type Primitive%20Component%20Object%20Reference) (OtherBodyIndex :type Integer) (bFromSweep :type Boolean) (SweepResult :type Hit%20Result%20Structure%20%28by%20ref%29))
  (bind _asmy_blaster_character (Utilities|Casting|CastToMyBlasterCharacter OtherActor))
  (if (not (Utilities|Enum|Equal(Enum) (Utilities|GetObjectName OtherComp) "InteractSphere"))
    (Pawn|Components|CharacterMovement|SetMovementMode (Variables|/Script/Engine.Character|GetCharacterMovement _asmy_blaster_character) "MOVE_Flying" 0)))

(event OnComponentEndOverlap(Box)
  (params (OverlappedComponent :type Primitive%20Component%20Object%20Reference) (OtherActor :type Actor%20Object%20Reference) (OtherComp :type Primitive%20Component%20Object%20Reference) (OtherBodyIndex :type Integer))
  (bind _asmy_blaster_character (Utilities|Casting|CastToMyBlasterCharacter OtherActor))
  (if (not (Utilities|Enum|Equal(Enum) (Utilities|GetObjectName OtherComp) "InteractSphere"))
    (Pawn|Components|CharacterMovement|SetMovementMode (Variables|/Script/Engine.Character|GetCharacterMovement _asmy_blaster_character) "MOVE_Walking" 0)))

(event OnComponentHit(Cube)
  (params (HitComponent :type Primitive%20Component%20Object%20Reference) (OtherActor :type Actor%20Object%20Reference) (OtherComp :type Primitive%20Component%20Object%20Reference) (NormalImpulse :type Vector :default "0, 0, 0") (Hit :type Hit%20Result%20Structure%20%28by%20ref%29))
  (bind _asmy_blaster_character (Utilities|Casting|CastToMyBlasterCharacter OtherActor))
  (if (not (Utilities|Enum|Equal(Enum) (Utilities|GetObjectName OtherComp) "InteractSphere"))
    (Class|PawnMovementComponent|AddInputVector (Variables|/Script/Engine.Character|GetCharacterMovement _asmy_blaster_character) (* (+ (* (Variables|Default|GetBackPush) (Math|Vector|MakeVector (.x (Math|Vector|Normalize (- (Transformation|GetActorLocation _asmy_blaster_character) (Transformation|GetActorLocation)))) (.y (Math|Vector|Normalize (- (Transformation|GetActorLocation _asmy_blaster_character) (Transformation|GetActorLocation)))) 0.0)) (Math|Vector|MakeVector 0.0 0.0 (Variables|Default|GetUpSpeed))) (Math|Vector|MakeVector 1.0 1.0 (Math|Float|Sign(Float) (.pitch (Transformation|GetWorldRotation (Variables|/Script/Blaster.BlasterCharacter|GetFirstPersonCamera _asmy_blaster_character)))))) false)))

(fn ConstructionScript
  (Transformation|SetWorldScale3D (Variables|Default|GetBox) (* (Transformation|GetWorldScale (Variables|Default|GetCube)) (LocalVariables|Getscale))))