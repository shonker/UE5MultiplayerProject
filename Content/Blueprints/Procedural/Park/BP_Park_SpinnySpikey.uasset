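; BP_Park_SpinnySpikey is a procedural park obstacle whose SpinnySpike component periodically spins in yaw through a timeline.
; BeginPlay offsets a start delay by the blaster player controller's server time, aligning the cycle to the server clock.
; A looping timer then triggers spins at intervals derived from the object name's last digit, which procedural generation keeps consistent.
; The spike's hit event is empty, leaving a character jump disconnected.
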(event OnComponentHit(SpinnySpike)
  (params (HitComponent :type Primitive%20Component%20Object%20Reference) (OtherActor :type Actor%20Object%20Reference) (OtherComp :type Primitive%20Component%20Object%20Reference) (NormalImpulse :type Vector :default "0, 0, 0") (Hit :type Hit%20Result%20Structure%20%28by%20ref%29)))

(event Custom|spin%20a%20lil
  (bind _spinnyspike (Variables|Default|GetSpinnySpike))
  (bind _returnvalue (Transformation|GetWorldRotation _spinnyspike))
  (bind _newtrack_0 (Timeline|setrotation PlayFromStart)
    (:Update
      (Transformation|SetWorldRotation _spinnyspike (Math|Rotator|MakeRotator (.roll _returnvalue) (.pitch _returnvalue) _newtrack_0) false false))))

(event Custom|CreateTimer
  (Utilities|Time|SetTimerbyEvent (delegate Custom|spin%20a%20lil) (+ (* (Math|Conversions|ToFloat(Integer) (Utilities|String|Right (Class|KismetSystemLibrary|GetPathName self) 1)) 2.0) 2e+01) true))

(event EventBeginPlay
  (bind _asbp_blaster_player_controller (Utilities|Casting|CastToBP_BlasterPlayerController (Game|GetPlayerController 0)))
  (bind _returnvalue (Class|BlasterPlayerController|GetServerTime _asbp_blaster_player_controller))
  (Utilities|Time|SetTimerbyEvent (delegate Custom|CreateTimer) (- (Variables|Default|Getbeginning%20wait) _returnvalue)))

(fn ConstructionScript)