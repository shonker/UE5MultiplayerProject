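; BP_Park_Horsey is a procedurally placed park horse whose animation playback is synced to server time in a multiplayer game.
; On BeginPlay it gets server time from the Blaster player controller and sets the Horsey component's playback position from it, without firing notifies.
; The last digit of the actor's path name, scaled down, offsets each instance, relying on consistent procedural naming to stagger horses identically everywhere.
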(event EventBeginPlay
  (bind _asbp_blaster_player_controller (Utilities|Casting|CastToBP_BlasterPlayerController (Game|GetPlayerController 0)))
  (bind _returnvalue (Class|BlasterPlayerController|GetServerTime _asbp_blaster_player_controller))
  (Components|Animation|SetPosition (Variables|Default|GetHorsey) (+ _returnvalue (* (Math|Conversions|ToFloat(Integer) (Utilities|String|Right (Class|KismetSystemLibrary|GetPathName self) 1)) 0.25)) false))

(event Collision|EventActorBeginOverlap
  (params (OtherActor :type Actor%20Object%20Reference)))

(event EventTick
  (params (DeltaSeconds :type Float%20%28single-precision%29)))

(fn ConstructionScript)