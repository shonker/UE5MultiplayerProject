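; BP_ParkPart_Square is a square park part Blueprint that, by its name and folder, serves as a piece for procedural park building.
; Its construction script fills OutputTransforms with the relative transform of the Output2 component alone.
; A disconnected array node holding the transforms of all four Output components remains in the graph, so the other three are not exposed through OutputTransforms.
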(fn ConstructionScript
  (Variables|Default|SetOutputTransforms (Utilities|Array|MakeArray (Transformation|GetRelativeTransform (Variables|Default|GetOutput2)))))