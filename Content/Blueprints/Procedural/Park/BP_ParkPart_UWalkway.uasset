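; BP_ParkPart_UWalkway is a U-walkway piece for procedural park generation.
; Its construction script stores the relative locations of four output components in OutputLocations, in the order Output, Output2, Output3, Output1.
; A random coin flip then destroys both the Topper and Legs components together, so instances vary between having both and having neither.
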(fn ConstructionScript
  (Variables|Default|SetOutputLocations (Utilities|Array|MakeArray (Variables|/Script/Engine.SceneComponent|GetRelativeLocation (Variables|Default|GetOutput)) (Variables|/Script/Engine.SceneComponent|GetRelativeLocation (Variables|Default|GetOutput2)) (Variables|/Script/Engine.SceneComponent|GetRelativeLocation (Variables|Default|GetOutput3)) (Variables|/Script/Engine.SceneComponent|GetRelativeLocation (Variables|Default|GetOutput1))))
  (if (Math|Random|RandomBool)
    (Components|DestroyComponent (Variables|Default|GetTopper))
    (Components|DestroyComponent (Variables|Default|GetLegs))))