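; Slide piece for the procedural park, which randomizes its color when play begins.
; Two coin flips either leave the mesh materials untouched or push their color scalar parameters toward red or blue.
; The construction script publishes the Output component's relative transform as the sole entry in OutputTransforms.
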(event EventBeginPlay
  (if (not (Math|Random|RandomBool))
    (if (Math|Random|RandomBool)
      (Rendering|Material|SetScalarParameterValueonMaterials (Variables|Default|GetSM_ParkPart) "Red" 1e+01)
      (Rendering|Material|SetScalarParameterValueonMaterials (Variables|Default|GetSM_ParkPart) "Green" 0.0)
      (else
        (Rendering|Material|SetScalarParameterValueonMaterials (Variables|Default|GetSM_ParkPart) "Green" 0.0)
        (Rendering|Material|SetScalarParameterValueonMaterials (Variables|Default|GetSM_ParkPart) "Blue" 1e+01)
        (Rendering|Material|SetScalarParameterValueonMaterials (Variables|Default|GetSM_ParkPart) "Red" 0.0)))))

(fn ConstructionScript
  (Variables|Default|SetOutputTransforms (Utilities|Array|MakeArray (Transformation|GetRelativeTransform (Variables|Default|GetOutput)))))