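; Procedural house room Blueprint that defines relative transforms, apparently as spawn points for house generation.
; The construction script appends the center output component's transform to a floor-center list and collects four wall output transforms into a floor-wall list.
; It derives middle-wall transforms by copying each floor-wall transform with a fixed upward Z offset.
; The event graph has no active logic.
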(event EventBeginPlay)

(event Collision|EventActorBeginOverlap
  (params (OtherActor :type Actor%20Object%20Reference)))

(event EventTick
  (params (DeltaSeconds :type Float%20%28single-precision%29)))

(fn ConstructionScript
  (Utilities|Array|Add (Variables|Default|GetFloorCenterOutputTransform) (Transformation|GetRelativeTransform (Variables|Default|GetCenterOutputTransform)))
  (bind _output_get (Variables|Default|SetFloorWallSpawnableTransforms (Utilities|Array|MakeArray (Transformation|GetRelativeTransform (Variables|Default|GetFloorWallOutputTransforms1)) (Transformation|GetRelativeTransform (Variables|Default|GetFloorWallOutputTransforms2)) (Transformation|GetRelativeTransform (Variables|Default|GetFloorWallOutputTransforms3)) (Transformation|GetRelativeTransform (Variables|Default|GetFloorWallOutputTransforms)))))
  (for _array_element _output_get
    (Utilities|Array|Add (Variables|Default|GetMiddleWallSpawnableTransforms) (Math|Transform|MakeTransform (Math|Vector|MakeVector (.x (.location _array_element)) (.y (.location _array_element)) (+ (.z (.location _array_element)) 273.0)) (.rotation _array_element) (.scale _array_element)))))