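; Procedural house wall piece with a destructible geometry collection and predefined placement slots for objects on the wall.
; The construction script hides the geometry collection and caches the relative transforms of arrow components into narrow-object and wide-object arrays, with the two wide slots reusing narrow-slot arrows.
; Activating the root component acts as the break trigger, activating the geometry collection, enabling physics simulation and making it visible.
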(event OnComponentActivated(DefaultRoot)
  (params (Component :type Actor%20Component%20Object%20Reference) (bReset :type Boolean))
  (bind _houseplot_normalwall_geometrycollection (Variables|Default|GetHousePlot_NormalWall_GeometryCollection))
  (Components|Activation|Activate _houseplot_normalwall_geometrycollection false)
  (Physics|SetSimulatePhysics _houseplot_normalwall_geometrycollection true)
  (Rendering|SetVisibility _houseplot_normalwall_geometrycollection true false))

(fn ConstructionScript
  (bind _arrow4 (Variables|Default|GetArrow4))
  (bind _arrow2 (Variables|Default|GetArrow2))
  (bind _returnvalue (Transformation|GetRelativeTransform _arrow4))
  (bind _returnvalue_2 (Transformation|GetRelativeTransform _arrow2))
  (Rendering|SetVisibility (Variables|Default|GetHousePlot_NormalWall_GeometryCollection) false false)
  (Variables|Default|SetNarrowObjectTransforms (Utilities|Array|MakeArray _returnvalue (Transformation|GetRelativeTransform (Variables|Default|GetArrow3)) _returnvalue_2 (Transformation|GetRelativeTransform (Variables|Default|GetArrow1)) (Transformation|GetRelativeTransform (Variables|Default|GetArrow)) (Transformation|GetRelativeTransform (Variables|Default|GetArrow5))))
  (Variables|Default|SetWideObjectTransforms (Utilities|Array|MakeArray _returnvalue_2 _returnvalue)))