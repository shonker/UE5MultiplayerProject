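; White table furniture Blueprint for the procedural house, defining transforms where objects can spawn.
; Its construction script runs the parent's script, then fills SpawnableObjectTransforms with the relative transforms of six Arrow components.
; The arrows act as placement markers, so the spawn transforms follow the component layout.
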(fn ConstructionScript
  (|CallParentFunction)
  (Variables|Default|SetSpawnableObjectTransforms (Utilities|Array|MakeArray (Transformation|GetRelativeTransform (Variables|Default|GetArrow1)) (Transformation|GetRelativeTransform (Variables|Default|GetArrow2)) (Transformation|GetRelativeTransform (Variables|Default|GetArrow3)) (Transformation|GetRelativeTransform (Variables|Default|GetArrow4)) (Transformation|GetRelativeTransform (Variables|Default|GetArrow5)) (Transformation|GetRelativeTransform (Variables|Default|GetArrow)))))