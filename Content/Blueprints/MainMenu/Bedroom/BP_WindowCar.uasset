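; BP_WindowCar is a main menu bedroom actor that fakes a car driving past the window with a moving RectLight.
; A randomly delayed, self-rescheduling timer fires Driveby, which snaps the light back to its relative origin and sets CarActive.
; Tick then slides the light along local negative Y by a fixed per-frame step, independent of delta time; CarActive is never cleared here.
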(event Custom|driveby
  (Transformation|SetRelativeLocation (Variables|Default|GetRectLight) "0, 0, 0" false false)
  (Utilities|Time|SetTimerbyEvent (delegate Custom|driveby) (Math|Random|RandomFloatinRange 3e+01 6e+01))
  (Variables|Default|SetCarActive true))

(event EventBeginPlay
  (Utilities|Time|SetTimerbyEvent (delegate Custom|driveby) (Math|Random|RandomFloatinRange 3e+01 6e+01)))

(event Collision|EventActorBeginOverlap
  (params (OtherActor :type Actor%20Object%20Reference)))

(event EventTick
  (params (DeltaSeconds :type Float%20%28single-precision%29))
  (Transformation|AddLocalOffset (Variables|Default|GetRectLight) (Math|Vector|MakeVector 0.0 (* (Math|Conversions|ToFloat(Boolean) (Variables|Default|GetCarActive)) -1e+01) 0.0) false false))

(fn ConstructionScript)