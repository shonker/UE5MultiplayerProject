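; Main menu bedroom actor that fakes a flickering TV glow and removes unwanted camera actors from the scene.
; On BeginPlay it stores the TV light's starting intensity and destroys every CameraActor that is not a BP_BedroomCamera.
; Each Tick randomly nudges the intensity up, down or not at all by a flicker coefficient.
; A looping timer periodically restores the starting intensity, keeping the random walk from drifting.
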(event Custom|ResetTv
  (Rendering|Components|Light|SetIntensity (Variables|Default|GetTVLight) (stale EventBeginPlay _output_get)))

(event EventBeginPlay
  (bind _output_get (Variables|Default|SetInitialIntensity (Variables|/Script/Engine.LightComponentBase|GetIntensity (Variables|Default|GetTVLight))))
  (Utilities|Time|SetTimerbyEvent (delegate Custom|ResetTv) 2.0 true)
  (bind _outactors (Actor|GetAllActorsOfClass "/Script/Engine.CameraActor"))
  (bind _array_element (Utilities|Array|ForEachLoopwithBreak _outactors)
    (:LoopBody
      (Utilities|Casting|CastToBP_BedroomCamera _array_element
        (:CastFailed
          (Actor|DestroyActor _array_element))))))

(event EventTick
  (params (DeltaSeconds :type Float%20%28single-precision%29))
  (bind _returnvalue (Math|Random|RandomBool))
  (bind _tvlight (Variables|Default|GetTVLight))
  (bind _tvflickercoefficient (Variables|Default|GetTvFlickerCoefficient))
  (bind _returnvalue_2 (Math|Conversions|ToInteger(Boolean) _returnvalue))
  (Rendering|Components|Light|SetIntensity _tvlight (+ (Variables|/Script/Engine.LightComponentBase|GetIntensity _tvlight) (* _tvflickercoefficient _returnvalue_2) (* (- _returnvalue_2 1) _tvflickercoefficient))))

(fn ConstructionScript)