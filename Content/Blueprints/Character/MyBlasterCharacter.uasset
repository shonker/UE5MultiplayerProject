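; Player character Blueprint handling first-person presentation and feedback for a shooter.
; On BeginPlay it hides locally controlled mesh parts with an invisible material, and crouch events move the FPS boom.
; Events drive a lazily created sniper scope widget with zoom animation and sound, and swap red/blue Niagara interaction dots.
; RadialBlur picks a timeline by whole-second duration to animate a Material Parameter Collection for damage blur.
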(event EventBeginPlay
  (CallFunction|LocallySetPlayerCharInvisible)
  (Components|Activation|SetActive (Variables|Default|GetNS_BlueDot) false false))

(event EventShowSniperScopeWidget
  (params (bShowScope :type Boolean))
  (CallFunction|SniperHUDWidget bShowScope))

(fn ConstructionScript)

(fn LocallySetPlayerCharInvisible
  (Variables|Default|SetCamera%20Boom (Variables|Default|GetCameraBoom))
  (if (Pawn|IsLocallyControlled)
    (Rendering|Material|SetMaterial (Variables|Character|GetMesh) 0 "/Game/CaydenAssets/SceneGirl/matsNtextures/M_Invisible.M_Invisible")
    (Rendering|Material|SetMaterial (Variables|Character|GetMesh) 3 "/Game/CaydenAssets/SceneGirl/matsNtextures/M_Invisible.M_Invisible")
    (Rendering|Material|SetMaterial (Variables|Character|GetMesh) 2 "/Game/CaydenAssets/SceneGirl/matsNtextures/M_Invisible.M_Invisible")
    (Rendering|Material|SetMaterial (Variables|Character|GetMesh) 4 "/Game/CaydenAssets/SceneGirl/matsNtextures/M_Invisible.M_Invisible")))

(fn SniperHUDWidget
  (params (InputPin :type Boolean))
  (Utilities|IsValid (Variables|Default|GetSniperScopeWidget)
    (:Is%20Valid
      _)
    (:Is%20Not%20Valid
      (bind _returnvalue (UserInterface|CreateWidget "/Game/Blueprints/HUD/WBP_SniperScope.WBP_SniperScope_C"))
      (bind _output_get (Variables|Default|SetSniperScopeWidget _returnvalue))
      (UserInterface|Viewport|AddtoViewport _output_get 0)))
  ;[1 1 1] zoom
  (if InputPin
    (Utilities|IsValid (Variables|Default|GetSniperScopeWidget)
      (:Is%20Valid
        (UserInterface|Animation|PlayAnimation (Variables|Default|GetSniperScopeWidget) (Variables|/Game/Blueprints/HUD/WBP_SniperScope.WBP_SniperScope_C|GetScopeZoomIn (Variables|Default|GetSniperScopeWidget)) 0.0 1 "Forward" 1.0 false)
        (Audio|PlaySound2D "/Game/Assets/MilitaryWeapSilver/Sound/SniperRifle/Cues/SniperRifle_ZoomIn_Cue.SniperRifle_ZoomIn_Cue" 1.0 1.0 0.0 0 0)))
    (else
      ;[1 1 1] unzoom
      (Utilities|IsValid (Variables|Default|GetSniperScopeWidget)
        (:Is%20Valid
          (UserInterface|Animation|PlayAnimation (Variables|Default|GetSniperScopeWidget) (Variables|/Game/Blueprints/HUD/WBP_SniperScope.WBP_SniperScope_C|GetScopeZoomIn (Variables|Default|GetSniperScopeWidget)) 0.0 1 "Reverse" 1.0 false)
          (Audio|PlaySound2D "/Game/Assets/MilitaryWeapSilver/Sound/SniperRifle/Cues/SniperRifle_ZoomOut_Cue.SniperRifle_ZoomOut_Cue" 1.0 1.0 0.0 0 0))))))

(event EventOnStartCrouch
  (params (HalfHeightAdjust :type Float%20%28single-precision%29) (ScaledHalfHeightAdjust :type Float%20%28single-precision%29))
  (Components|MoveComponentTo (Variables|Default|GetFPSBoom) "0, 0,80.000000" "0, 0, 0" false false 0.2 false))

(event EventOnEndCrouch
  (params (HalfHeightAdjust :type Float%20%28single-precision%29) (ScaledHalfHeightAdjust :type Float%20%28single-precision%29))
  (Components|MoveComponentTo (Variables|Default|GetFPSBoom) "0, 0,115.000000" "0, 0, 0" false false 0.2 false))

(event EventRadialBlur
  (params (Intensity :type Float%20%28single-precision%29) (Duration :type Float%20%28single-precision%29))
  (Utilities|IsValid (Variables|Default|GetPostProcessVol)
    (:Is%20Valid
      _)
    (:Is%20Not%20Valid
      (bind _outactors (Actor|GetAllActorsOfClass "/Script/Engine.PostProcessVolume"))
      (Variables|Default|SetPostProcessVol (Utilities|Array|Get(acopy) _outactors))))
  (Variables|Default|SetTargBlur (/ Intensity 3.0))
  (switch int (Math|Conversions|ToInteger(Byte) (Class|KismetMathLibrary|FFloor64 Duration))
    (:Default
      ;[1 1 1] long blur
      (bind _newtrack_0 (Timeline|EnterRadialBlurTimeline PlayFromStart)
        (:Update
          (Rendering|Material|SetScalarParameterValue "/Game/CaydenAssets/Materials/RadialBlur/MPC_RadialBlur.MPC_RadialBlur" "Blur" _newtrack_0 :!class /Script/Engine.KismetMaterialLibrary)
          (Rendering|Material|SetScalarParameterValue "/Game/CaydenAssets/Materials/RadialBlur/MPC_RadialBlur.MPC_RadialBlur" "Blur Radius" _newtrack_0 :!class /Script/Engine.KismetMaterialLibrary)
          (Rendering|Material|SetScalarParameterValue "/Game/CaydenAssets/Materials/RadialBlur/MPC_RadialBlur.MPC_RadialBlur" "Density" (* _newtrack_0 4.0) :!class /Script/Engine.KismetMaterialLibrary))))
    (:0
      ;[1 1 1] short blur
      (bind _newtrack_0_2 (Timeline|Timeline_1 PlayFromStart)
        (:Update
          (Rendering|Material|SetScalarParameterValue "/Game/CaydenAssets/Materials/RadialBlur/MPC_RadialBlur.MPC_RadialBlur" "Blur" _newtrack_0_2 :!class /Script/Engine.KismetMaterialLibrary)
          (Rendering|Material|SetScalarParameterValue "/Game/CaydenAssets/Materials/RadialBlur/MPC_RadialBlur.MPC_RadialBlur" "Blur Radius" _newtrack_0_2 :!class /Script/Engine.KismetMaterialLibrary)
          (Rendering|Material|SetScalarParameterValue "/Game/CaydenAssets/Materials/RadialBlur/MPC_RadialBlur.MPC_RadialBlur" "Density" (* _newtrack_0_2 4.0) :!class /Script/Engine.KismetMaterialLibrary)
          (Development|PrintString "Hello"))))
    (:1
      ;[1 1 1] med blur
      (bind _newtrack_0_3 (Timeline|Timeline_0 PlayFromStart)
        (:Update
          (Rendering|Material|SetScalarParameterValue "/Game/CaydenAssets/Materials/RadialBlur/MPC_RadialBlur.MPC_RadialBlur" "Blur" _newtrack_0_3 :!class /Script/Engine.KismetMaterialLibrary)
          (Rendering|Material|SetScalarParameterValue "/Game/CaydenAssets/Materials/RadialBlur/MPC_RadialBlur.MPC_RadialBlur" "Blur Radius" _newtrack_0_3 :!class /Script/Engine.KismetMaterialLibrary)
          (Rendering|Material|SetScalarParameterValue "/Game/CaydenAssets/Materials/RadialBlur/MPC_RadialBlur.MPC_RadialBlur" "Density" (* _newtrack_0_3 4.0) :!class /Script/Engine.KismetMaterialLibrary))))
    (:2
      (Timeline|EnterRadialBlurTimeline PlayFromStart))))

(event EventChangeInteractionDotColor
  (params (bInteractionDetected :type Boolean))
  (bind _ns_reddot (Variables|Default|GetNS_RedDot))
  (bind _ns_bluedot (Variables|Default|GetNS_BlueDot))
  (if bInteractionDetected
    (Components|Activation|SetActive _ns_bluedot true false)
    (Components|Activation|SetActive _ns_reddot false false)
    (else
      (Components|Activation|SetActive _ns_reddot true false)
      (Components|Activation|SetActive _ns_bluedot false false))))