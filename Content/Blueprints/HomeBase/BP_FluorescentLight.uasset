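; BP_FluorescentLight is a fluorescent light fixture for the home base that lights up after a delay.
; BeginPlay creates a dynamic bulb material on the cube mesh with its emissiveness at zero.
; TurnOn starts a one-shot timer of LightTimer length, which then sets a random emissive strength and plays a switch sound at the fixture.
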(event Custom|TurnOn
  (Utilities|Time|SetTimerbyEvent (delegate Custom|CustomEvent_0) (Variables|Default|GetLightTimer)))

(event Custom|CustomEvent_0
  (Rendering|Material|SetScalarParameterValue (stale EventBeginPlay _returnvalue) "Emissiveness" (* (Math|Random|RandomFloat) 1e+01) :!class /Script/Engine.MaterialInstanceDynamic)
  (Audio|PlaySoundatLocation "/Engine/VREditor/Sounds/UI/Flashlight_Switch.Flashlight_Switch" (Transformation|GetWorldLocation (Variables|Default|GetDefaultSceneRoot)) "0, 0, 0" 1.0 1.0 0.0 0 0 0 0))

(event EventBeginPlay
  (bind _returnvalue (Rendering|Material|CreateDynamicMaterialInstance (Variables|Default|GetFluorescentLight_Cube_001) 1 "/Game/CaydenAssets/HomeBase/FluorescentLights/MI_Bulb.MI_Bulb" "None" :!class /Script/Engine.PrimitiveComponent))
  (Rendering|Material|SetScalarParameterValue _returnvalue "Emissiveness" 0.0 :!class /Script/Engine.MaterialInstanceDynamic))

(fn ConstructionScript)