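; BP_Knight is a home base knight that gives sound and camera feedback as a sword is pulled out.
; On BeginPlay it hands itself to its mesh's ABP_Knight anim instance.
; Sword button presses start a deep rumble, which stops on release or drag-off.
; SwordScreenShake scales a world camera shake's radii by intensity and, near intensity three, swaps the rumble for a pullout cue unless one already exists.
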(event EventBPSwordButtonPressed
  (bind _returnvalue (Audio|SpawnSoundatLocation "/Game/CaydenAssets/Sounds/Sounds/LowRumble/Cue_DeepRumble.Cue_DeepRumble" (Transformation|GetActorLocation self) "0, 0, 0" 1.0 1.0 0.0 0 0))
  (bind _output_get (Variables|Default|SetLowRumbleSound _returnvalue)))

(event EventBPSwordButtonDraggedOff
  (Audio|Components|Audio|Stop (stale EventBPSwordButtonPressed _output_get)))

(event EventBPSwordButtonReleased
  (Audio|Components|Audio|Stop (stale EventBPSwordButtonPressed _output_get)))

(event EventSwordScreenShake
  (params (ShakeIntensityUpToFour :type Float%20%28single-precision%29))
  (bind _returnvalue (/ ShakeIntensityUpToFour 3.0))
  (bind _radius (Variables|Default|GetRadius))
  (Camera|PlayWorldCameraShake "/Game/Blueprints/HomeBase/BP_SwordCameraShake.BP_SwordCameraShake_C" (Transformation|GetActorLocation) (* (* _returnvalue 2.0) _radius) (* (* _returnvalue 1e+01) _radius))
  (if (>= ShakeIntensityUpToFour 2.99)
    (Utilities|IsValid (stale _output_get)
      (:Is%20Not%20Valid
        (bind _returnvalue_2 (Audio|SpawnSoundatLocation "/Game/CaydenAssets/Sounds/Sounds/LowRumble/Cue_SwordPullout.Cue_SwordPullout" (Transformation|GetActorLocation self) "0, 0, 0" 1.0 1.0 0.0 0 0))
        (bind _output_get (Variables|Default|SetSwordPulloutCue _returnvalue_2))
        (Audio|Components|Audio|Stop (stale EventBPSwordButtonPressed _output_get))))))

(event EventBeginPlay
  (bind _asabp_knight (Utilities|Casting|CastToABP_Knight (Components|SkeletalMesh|GetAnimInstance (Variables|Default|GetKnightMesh))))
  (Variables|/Game/CaydenAssets/HomeBase/Knight/ABP_Knight.ABP_Knight_C|SetAs%20BP%20Knight _asabp_knight self)
  (Development|PrintString "knight cast succeeded"))

(fn ConstructionScript)