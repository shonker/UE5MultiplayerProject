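; BP_HomeBase is the home base Blueprint, which controls the base's eight fluorescent lights.
; ActivateLights gathers the BP_FluorescentLight child actors and turns them on, using a toggling boolean added as a float to increase LightTimer on every other light, staggering activation in pairs.
; RedLights loops over the same stored array to turn every light red, so it relies on ActivateLights having filled it.
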(event EventActivateLights
  (bind _output_get (Variables|Default|SetFluLights (Utilities|Array|MakeArray (Variables|Default|GetBP_FluorescentLight) (Variables|Default|GetBP_FluorescentLight1) (Variables|Default|GetBP_FluorescentLight2) (Variables|Default|GetBP_FluorescentLight3) (Variables|Default|GetBP_FluorescentLight4) (Variables|Default|GetBP_FluorescentLight5) (Variables|Default|GetBP_FluorescentLight6) (Variables|Default|GetBP_FluorescentLight7))))
  (for _array_element _output_get
    (bind _asbp_fluorescent_light (Utilities|Casting|CastToBP_FluorescentLight (Variables|/Script/Engine.ChildActorComponent|GetChildActor _array_element)))
    ;[1 1 1] activate two at a time
    (Variables|Default|SetbTimerIncrement (not (Variables|Default|GetbTimerIncrement)))
    (bind _output_get_2 (Variables|Default|SetFluLightTime (+ (Variables|Default|GetFluLightTime) (Math|Conversions|ToFloat(Boolean) (Variables|Default|GetbTimerIncrement)))))
    (Variables|/Game/Blueprints/HomeBase/BP_FluorescentLight.BP_FluorescentLight_C|SetLightTimer _asbp_fluorescent_light _output_get_2)
    (Default|Turnon _asbp_fluorescent_light)))

(event EventRedLights
  (for _array_element (stale EventActivateLights _output_get)
    (bind _asbp_fluorescent_light (Utilities|Casting|CastToBP_FluorescentLight (Variables|/Script/Engine.ChildActorComponent|GetChildActor _array_element)))
    (Default|TurnRed _asbp_fluorescent_light)))

(fn ConstructionScript)