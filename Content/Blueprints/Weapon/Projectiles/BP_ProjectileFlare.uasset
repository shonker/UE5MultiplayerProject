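; BP_ProjectileFlare is a flare projectile with a flickering point light.
; On BeginPlay a timeline starts and sets the projectile movement component's max speed to the Spd variable scaled by the timeline track, shaping its speed over time.
; Every Tick randomizes the point light between half and full of the Intensity variable to create the flicker.
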(event EventBeginPlay
  (Utilities|FlowControl|Sequence
    (:then_0
      (bind _newtrack_0 (Timeline|Timeline_0 Play)
        (:Update
          (Variables|/Script/Engine.ProjectileMovementComponent|SetMaxSpeed (Variables|Default|GetProjectileMovementComponent) (* (Variables|Default|GetSpd) _newtrack_0)))))))

(event Collision|EventActorBeginOverlap
  (params (OtherActor :type Actor%20Object%20Reference)))

(event EventTick
  (params (DeltaSeconds :type Float%20%28single-precision%29))
  (Rendering|Components|Light|SetIntensity (Variables|Default|GetPointLight) (* (Variables|Default|Getintensity) (Math|Random|RandomFloatinRange 0.5 1.0))))

(fn ConstructionScript)