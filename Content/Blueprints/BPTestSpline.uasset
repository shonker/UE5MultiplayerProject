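; Test spline actor that builds a chain of deformed meshes along its spline in the construction script, with collision enabled.
; It places one spline mesh per SectionLength of spline, which AllowScaling takes from actor X scale.
; Tangents come from length-clamped spline locations rather than spline tangents.
; The MustBeFullLengthMeshes branch only adds a single unconfigured component, and the event graph is empty.
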(event EventBeginPlay)

(event Collision|EventActorBeginOverlap
  (params (OtherActor :type Actor%20Object%20Reference)))

(event EventTick
  (params (DeltaSeconds :type Float%20%28single-precision%29)))

(fn ConstructionScript
  (bind _splinecomponent (Variables|Default|GetSplineComponent))
  (bind _splinecomponent_2 (Variables|Default|GetSplineComponent))
  (if (LocalVariables|GetbAllowScaling)
    (LocalVariables|SetSectionLength (.x (Transformation|GetActorScale3D))))
  (if (LocalVariables|GetbMustBeFullLengthMeshes)
    (for _index (range 0 0)
      (LocalVariables|SetLoopIndex _index)
      (AddComponent|AddSplineMeshComponent false))
    (else
      (for _index_2 (range 0 (Math|Float|Truncate (/ (Spline|GetSplineLength (Variables|Default|GetSplineComponent)) (LocalVariables|GetSectionLength))))
        (LocalVariables|SetLoopIndex _index_2)
        (bind _returnvalue (AddComponent|AddSplineMeshComponent false))
        (Components|StaticMesh|SetStaticMesh _returnvalue (Variables|Default|GetSplineMesh))
        (SplineMesh|SetForwardAxis _returnvalue "X" true)
        (SplineMesh|SetStartandEnd _returnvalue (Spline|GetLocationatDistanceAlongSpline _splinecomponent (* (LocalVariables|GetLoopIndex) (LocalVariables|GetSectionLength)) "Local") (Math|Vector|ClampVectorSize (Spline|GetLocationatDistanceAlongSpline _splinecomponent (* (LocalVariables|GetLoopIndex) (LocalVariables|GetSectionLength)) "Local") 0.0 (LocalVariables|GetSectionLength)) (Spline|GetLocationatDistanceAlongSpline _splinecomponent_2 (* (+ (LocalVariables|GetLoopIndex) 1) (LocalVariables|GetSectionLength)) "Local") (Math|Vector|ClampVectorSize (Spline|GetLocationatDistanceAlongSpline _splinecomponent_2 (* (+ (LocalVariables|GetLoopIndex) 1) (LocalVariables|GetSectionLength)) "Local") 0.0 (LocalVariables|GetSectionLength)) true :!class /Script/Engine.SplineMeshComponent)
        (Collision|SetCollisionEnabled _returnvalue "QueryAndPhysics")))))