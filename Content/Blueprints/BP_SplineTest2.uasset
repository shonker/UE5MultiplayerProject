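; Test actor that builds a chain of colliding spline meshes along its SplineComponent at BeginPlay.
; It divides the spline by SectionLength, optionally taken from actor X scale, and places one mesh per section.
; Tangents come from clamped spline locations rather than spline tangents, and the components use manual attachment without being attached.
; The MustBeFullLengthMeshes branch only adds an unconfigured component; the construction-script copy never runs.
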(event Custom|CustomEvent_0)

(event EventBeginPlay
  (bind _splinecomponent (Variables|Default|GetSplineComponent))
  (bind _splinecomponent_2 (Variables|Default|GetSplineComponent))
  (if (Variables|Default|GetbAllowScaling)
    (Variables|Default|SetSectionLength (.x (Transformation|GetActorScale3D))))
  (if (Variables|Default|GetbMustBeFullLengthMeshes)
    (for _index (range 0 0)
      (Variables|Default|SetLoopIndex _index)
      (AddComponent|AddSplineMeshComponent false))
    (else
      (for _index_2 (range 0 (Math|Float|Truncate (/ (Spline|GetSplineLength (Variables|Default|GetSplineComponent)) (Variables|Default|GetSectionLength))))
        (Variables|Default|SetLoopIndex _index_2)
        (bind _returnvalue (AddComponent|AddSplineMeshComponent true))
        (Components|StaticMesh|SetStaticMesh _returnvalue (Variables|Default|GetSplineMesh))
        (SplineMesh|SetForwardAxis _returnvalue "X" true)
        (SplineMesh|SetStartandEnd _returnvalue (Spline|GetLocationatDistanceAlongSpline _splinecomponent (* (Variables|Default|GetLoopIndex) (Variables|Default|GetSectionLength)) "Local") (Math|Vector|ClampVectorSize (Spline|GetLocationatDistanceAlongSpline _splinecomponent (* (Variables|Default|GetLoopIndex) (Variables|Default|GetSectionLength)) "Local") 0.0 (Variables|Default|GetSectionLength)) (Spline|GetLocationatDistanceAlongSpline _splinecomponent_2 (* (+ (Variables|Default|GetLoopIndex) 1) (Variables|Default|GetSectionLength)) "Local") (Math|Vector|ClampVectorSize (Spline|GetLocationatDistanceAlongSpline _splinecomponent_2 (* (+ (Variables|Default|GetLoopIndex) 1) (Variables|Default|GetSectionLength)) "Local") 0.0 (Variables|Default|GetSectionLength)) true :!class /Script/Engine.SplineMeshComponent)
        (Collision|SetCollisionEnabled _returnvalue "QueryAndPhysics")))))

(fn ConstructionScript)