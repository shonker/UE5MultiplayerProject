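; BP_SplineHell is an unfinished spline-mesh actor meant to tile a mesh along a spline, but all its logic is disconnected.
; BeginPlay, the custom event and the construction script are empty.
; The orphaned loop cuts the spline into SectionLength segments, optionally taken from X scale, adding colliding spline meshes with tangents derived from clamped locations.
; The full-length branch only adds one unconfigured component.
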(event Custom|CustomEvent_0)

(event EventBeginPlay)

(fn ConstructionScript)